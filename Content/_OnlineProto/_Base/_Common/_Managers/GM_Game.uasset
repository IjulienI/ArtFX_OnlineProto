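; Game mode for an online hide-and-seek match that assigns Seeker and Hider roles and spawns the players.
; BeginPlay sorts custom player starts into seeker and hider lists.
; PostLogin retries each tick until the GameInstance is valid, and once controllers match its player count, randomly picks unique seekers by index.
; It flags their PlayerStates, spawns and possesses each role's pawn at a random matching start, then updates GameState widget visibility.
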(event EventBeginPlay
  (|CallParentFunction)
  (bind _outactors (Actor|GetAllActorsOfClass "/Game/_OnlineProto/_Base/_Common/Actor/BP_CustomPlayerStart.BP_CustomPlayerStart_C"))
  (for _array_element _outactors
    (if (Variables|/Game/_OnlineProto/_Base/_Common/Actor/BP_CustomPlayerStart.BP_CustomPlayerStart_C|GetbSeeker _array_element)
      (Utilities|Array|Add (Variables|Default|GetSeekerStarts) _array_element)
      (else
        (Utilities|Array|Add (Variables|Default|GetHiderStart) _array_element)))))

(event EventPostLogin
  (params (NewPlayer :type Player%20Controller%20Object%20Reference))
  (|CallParentFunction NewPlayer)
  (Utilities|IsValid (Variables|Default|GetGameInstance) :!label _label
    (:Is%20Valid
      (if (== (Variables|/Game/_OnlineProto/_Base/_Common/_Managers/GI_OnlineProto.GI_OnlineProto_C|GetPlayerCount (Variables|Default|GetGameInstance)) (Utilities|Array|Length (Variables|Default|GetPlayerControllers)))
        (CallFunction|GetSeekers)
        (CallFunction|SpawnPlayer)
        (bind _asgs_game (Utilities|Casting|CastToGS_Game (Game|GetGameState)))
        (Default|SetWidgetVisibility _asgs_game)))
    (:Is%20Not%20Valid
      (Utilities|FlowControl|DelayUntilNextTick)
      (goto _label))))

(fn ConstructionScript
  (|CallParentFunction))

(fn GetSeekers
  (while (!= (Variables|/Game/_OnlineProto/_Base/_Common/_Managers/GI_OnlineProto.GI_OnlineProto_C|GetSeekerCount (Variables|Default|GetGameInstance)) (Utilities|Array|Length (Variables|Default|GetRandomSeeker)))
    (LocalVariables|SetTempSeeker (Math|Random|RandomIntegerinRange 0 (- (Variables|/Game/_OnlineProto/_Base/_Common/_Managers/GI_OnlineProto.GI_OnlineProto_C|GetPlayerCount (Variables|Default|GetGameInstance)) 1)))
    (LocalVariables|SetbInValid false)
    (for _array_element (Variables|Default|GetRandomSeeker)
      (if (== (LocalVariables|GetTempSeeker) _array_element)
        (LocalVariables|SetbInValid true)))
    (if (not (LocalVariables|GetbInValid))
      (Utilities|Array|Add (Variables|Default|GetRandomSeeker) (LocalVariables|GetTempSeeker))))
  (return))

(fn SpawnPlayer
  (for (_array_element _array_index) (Variables|Default|GetPlayerControllers)
    (LocalVariables|SetCurrentController _array_element)
    (for _array_element_2 (Variables|Default|GetRandomSeeker)
      (if (== _array_element_2 _array_index)
        (bind _asps_game (Utilities|Casting|CastToPS_Game (Variables|/Script/Engine.Controller|GetPlayerState (LocalVariables|GetCurrentController))))
        (Variables|/Game/_OnlineProto/_Base/_Common/_Managers/PS_Game.PS_Game_C|SetbSeeker _asps_game true)))
    (bind _asps_game_2 (Utilities|Casting|CastToPS_Game (Variables|/Script/Engine.Controller|GetPlayerState (LocalVariables|GetCurrentController))))
    (if (Variables|/Game/_OnlineProto/_Base/_Common/_Managers/PS_Game.PS_Game_C|GetbSeeker _asps_game_2)
      (bind _returnvalue (Game|SpawnActorfromClass "/Game/_OnlineProto/_Base/_Common/Character/BP_Seeker.BP_Seeker_C" (Transformation|GetActorTransform (.OutItem (Utilities|Array|Random (Variables|Default|GetSeekerStarts)))) "Undefined" "MultiplyWithRoot" 0 0))
      (Pawn|Possess (LocalVariables|GetCurrentController) _returnvalue)
      (else
        (bind _returnvalue_2 (Game|SpawnActorfromClass "/Game/_OnlineProto/_Base/_Common/Character/BP_Hider.BP_Hider_C" (Transformation|GetActorTransform (.OutItem (Utilities|Array|Random (Variables|Default|GetHiderStart)))) "Undefined" "MultiplyWithRoot" 0 0))
        (Pawn|Possess (LocalVariables|GetCurrentController) _returnvalue_2))))
  (return))