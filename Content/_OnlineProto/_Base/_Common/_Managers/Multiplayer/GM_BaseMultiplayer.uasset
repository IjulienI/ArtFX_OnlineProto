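; GM_BaseMultiplayer is a base multiplayer Game Mode that tracks connected player controllers and supports player count queries and kicking by index.
; PostLogin and OnLogout update the controller array, then trigger a player list refresh on GS_BaseMultiplayer, retrying each tick until the Game State is valid.
; KickPlayer delegates to CKickPlayer on the indexed PC_BaseMultiplayer.
; BeginPlay caches the GI_OnlineProto Game Instance.
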(event Custom|UpdatePlayerList
  (bind _returnvalue (Game|GetGameState))
  (Utilities|IsValid _returnvalue :!label _label
    (:Is%20Valid
      (bind _asgs_base_multiplayer (Utilities|Casting|CastToGS_BaseMultiplayer _returnvalue))
      (Default|UpdatePlayerList _asgs_base_multiplayer))
    (:Is%20Not%20Valid
      (Utilities|FlowControl|DelayUntilNextTick)
      (goto _label))))

(event EventBeginPlay
  (bind _asgi_online_proto (Utilities|Casting|CastToGI_OnlineProto (Game|GetGameInstance)))
  (Variables|Default|SetGameInstance _asgi_online_proto))

(event EventPostLogin
  (params (NewPlayer :type Player%20Controller%20Object%20Reference))
  (Utilities|Array|Add (Variables|Default|GetPlayerControllers) NewPlayer)
  (CallFunction|UpdatePlayerList))

(event EventOnLogout
  (params (ExitingController :type Controller%20Object%20Reference))
  (Utilities|Array|RemoveItem (Variables|Default|GetPlayerControllers) ExitingController)
  (CallFunction|UpdatePlayerList))

(fn ConstructionScript)

(fn KickPlayer
  (params (ID :type Integer))
  (bind _aspc_base_multiplayer (Utilities|Casting|CastToPC_BaseMultiplayer (Utilities|Array|Get(acopy) (Variables|Default|GetPlayerControllers) ID)))
  (Default|CKickPlayer _aspc_base_multiplayer))

(fn GetPlayerCount
  (return (Utilities|Array|Length (Variables|Default|GetPlayerControllers))))