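; Base character for an online prop-hunt game, handling interaction, sprint, damage and sounds, with empty shoot, prop-transformation and rotation-lock stubs.
; BeginPlay waits for PlayerState, caches references and starts a looping timer on Authority.
; A camera sphere trace highlights interactibles, excluding props for Seekers.
; S_/MC_ event pairs relay interaction, sprint and sounds, including random DT_Sounds picks, while damage goes to the PlayerState.
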(event Custom|S_Interact
  (bind _camera (Variables|Default|GetCamera))
  (bind _returnvalue (Transformation|GetWorldLocation _camera))
  ;[1 1 1] Base Interact
  (CallFunction|MCInteract _returnvalue (+ _returnvalue (* (Math|Vector|GetForwardVector _camera) 6e+02)) 15.0))

(event Custom|S_Sprint
  (params (bSprint :type Boolean))
  ;[1 1 1] Sprint
  (CallFunction|MCSprint bSprint))

(event Custom|PlayRandonSound
  ;[1 1 1] Play Random sound
  (bind _outrownames (DataTable|GetDataTableRowNames "/Game/_OnlineProto/_Base/Sounds/DT_Sounds.DT_Sounds"))
  (bind _returnvalue (Utilities|GetDataTableRow "/Game/_OnlineProto/_Base/Sounds/DT_Sounds.DT_Sounds" (.OutItem (Utilities|Array|Random _outrownames)))
    (:then
      (CallFunction|SPlaySoundAttached (.Sound (Utilities|Struct|BreakSTRUCT_Sound _returnvalue)) 0 true))))

(event Custom|MC_Interact
  (params (Start :type Vector) (End :type Vector) (Radius :type Float%20%28single-precision%29))
  ;[1 1 1] Base Interact
  (bind (_outhit _returnvalue) (Collision|SphereTraceByChannel Start End Radius "TraceTypeQuery1" false 0 "ForDuration"))
  (if _returnvalue
    (if (Utilities|DoesObjectImplementInterface (.HitActor (Collision|BreakHitResult _outhit)) "/Game/_OnlineProto/_Base/_Common/Interfaces/BPI_Interactible.BPI_Interactible_C")
      (Class|BPIInteractible|Interact(Message) (.HitActor (Collision|BreakHitResult _outhit)) self))))

(event Custom|DetectOverlapInteractor
  (bind _camera (Variables|Default|GetCamera))
  (bind _returnvalue (Transformation|GetWorldLocation _camera))
  ;[1 1 1] Detect interactible
  (Utilities|IsValid (Variables|Default|GetPlayerControllerRef)
    (:Is%20Valid
      (bind (_outhit _returnvalue_2) (Collision|SphereTraceByChannel _returnvalue (+ _returnvalue (* (Math|Vector|GetForwardVector _camera) 6e+02)) 15.0 "TraceTypeQuery1" false 0 "None" true "(R=1.000000,G=0.000000,B=0.000000,A=1.000000)" "(R=0.000000,G=1.000000,B=0.000000,A=1.000000)" 0.1))
      (if _returnvalue_2
        (if (Actor|ActorHasTag (.HitActor (Collision|BreakHitResult _outhit)) "Prop")
          (if (not (Variables|/Game/_OnlineProto/_Base/_Common/_Managers/PS_Game.PS_Game_C|GetbSeeker (Variables|Default|GetPlayerStateRef)))
            (if (Utilities|DoesObjectImplementInterface (.HitActor (Collision|BreakHitResult _outhit)) "/Game/_OnlineProto/_Base/_Common/Interfaces/BPI_Interactible.BPI_Interactible_C") :!label _label
              (Variables|Default|SetLastSelectedObject (.HitActor (Collision|BreakHitResult _outhit)))
              (Default|SelectObject (Variables|Default|GetPlayerControllerRef) true)
              (else
                (Default|SelectObject (Variables|Default|GetPlayerControllerRef) false :!label _label_2)))
            (else
              (goto _label_2)))
          (else
            (goto _label)))
        (else
          (Default|SelectObject (Variables|Default|GetPlayerControllerRef) false))))))

(event Custom|MC_Sprint
  (params (bSprint :type Boolean))
  ;[1 1 1] Sprint
  (Variables|/Script/Engine.CharacterMovementComponent|SetMaxWalkSpeed (Variables|Character|GetCharacterMovement) (select bSprint 8e+02 6e+02)))

(event Custom|S_Shoot
  ;[1 1 1] Shoot event
)

(event Custom|S_PlaySoundAttached
  (params (Sound :type Sound%20Base%20Object%20Reference) (AttachToComponent :type Scene%20Component%20Object%20Reference) (bSelf :type Boolean))
  ;[1 1 1] Play sound attached
  (CallFunction|MCPlaySoundAttached Sound (select bSelf (Variables|Character|GetMesh) AttachToComponent)))

(event Custom|MC_PlaySoundAttached
  (params (Sound :type Sound%20Base%20Object%20Reference) (AttachToComponent :type Scene%20Component%20Object%20Reference))
  ;[1 1 1] Play sound attached
  (Utilities|IsValid (Variables|Default|GetLastSound)
    (:Is%20Valid
      (Audio|Components|Audio|Stop (Variables|Default|GetLastSound))
      (Components|DestroyComponent (Variables|Default|GetLastSound)))
    (:Is%20Not%20Valid
      _))
  (bind _returnvalue (Audio|SpawnSoundAttached Sound AttachToComponent "None" "0, 0, 0" "0, 0, 0" "KeepRelativeOffset" false 1.0 1.0 0.0 "/Game/_OnlineProto/_Base/Sounds/SA_BaseAttenuation.SA_BaseAttenuation" 0))
  (Variables|Default|SetLastSound _returnvalue))

(event Custom|S_PlaySoundAtLocation
  (params (Sound :type Sound%20Base%20Object%20Reference) (Location :type Vector))
  ;[1 1 1] Play sound At location
  (CallFunction|MCPlaySoundatLocation Sound Location))

(event Custom|MC_PlaySoundAtLocation
  (params (Sound :type Sound%20Base%20Object%20Reference) (Location :type Vector))
  ;[1 1 1] Play sound At location
  (Audio|PlaySoundatLocation Sound Location "0, 0, 0" 1.0 1.0 0.0 0 0 0 0))

(event Game|Damage|EventAnyDamage
  (params (Damage :type Float%20%28single-precision%29) (DamageType :type Damage%20Type%20Object%20Reference) (InstigatedBy :type Controller%20Object%20Reference) (DamageCauser :type Actor%20Object%20Reference))
  ;[1 1 1] ApplyDamages
  (Default|GetDamage (Variables|Default|GetPlayerStateRef) Damage))

(event EventBeginPlay
  (bind _playerstate (Variables|GetPlayerState))
  ;[1 1 1] if own client, create loop
  (Utilities|IsValid _playerstate :!label _label
    (:Is%20Valid
      (bind _asps_game (Utilities|Casting|CastToPS_Game _playerstate))
      (Variables|Default|SetPlayerStateRef _asps_game)
      (bind _aspc_game (Utilities|Casting|CastToPC_Game (Game|GetPlayerController 0)))
      (Variables|Default|SetPlayerControllerRef _aspc_game)
      (switch Utilities|FlowControl|Switch|SwitchonENetRole (Networking|GetLocalRole)
        (:ROLE_Authority
          (Utilities|Time|SetTimerbyEvent (EventDispatchers|CreateEvent :!event Custom|DetectOverlapInteractor) 0.1 true))))
    (:Is%20Not%20Valid
      (Utilities|FlowControl|DelayUntilNextTick)
      (goto _label))))

(fn ConstructionScript)

(fn PropTransformation
  (params (Mesh :type Static%20Mesh%20Object%20Reference) (Offset :type Vector))
  (return))

(fn LockRotation
  (return))