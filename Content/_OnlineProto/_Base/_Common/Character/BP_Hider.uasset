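; BP_Hider is the hider character for a prop-hunt style mode, able to disguise itself as a prop.
; PropTransformation hides the character mesh, applies the prop to a static mesh, shrinks the capsule, repositions prop and spring arm from offset and bounds, and draws a debug sphere.
; LockRotation routes through a server event to a multicast that toggles controller yaw rotation.
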(event Custom|S_LockRotation
  (CallFunction|MCLockRotation))

(event Custom|MC_LockRotation
  (Variables|Default|SetbUseControllerRotationYaw (not (Variables|Default|GetbUseControllerRotationYaw))))

(fn ConstructionScript
  (|CallParentFunction))

(fn PropTransformation
  (params (Mesh :type Static%20Mesh%20Object%20Reference) (Offset :type Vector :default "0, 0, 0"))
  (bind _staticmesh (Variables|Default|GetStaticMesh))
  (bind _springarm (Variables|Default|GetSpringArm))
  (bind _capsulecomponent (Variables|Default|GetCapsuleComponent))
  (bind _relativelocation (Variables|/Script/Engine.SceneComponent|GetRelativeLocation _springarm))
  (bind _relativelocation_2 (Variables|/Script/Engine.SceneComponent|GetRelativeLocation _staticmesh))
  (Development|SetHiddeninGame (Variables|Character|GetMesh) true false)
  (Components|StaticMesh|SetStaticMesh (Variables|Default|GetStaticMesh) Mesh)
  (Components|Capsule|SetCapsuleRadius _capsulecomponent 15.0 true)
  (Components|Capsule|SetCapsuleHalfHeight _capsulecomponent 15.0 true)
  (Transformation|SetRelativeLocation _staticmesh (Math|Vector|MakeVector (.x _relativelocation_2) (.y _relativelocation_2) (- (* (Variables|/Script/Engine.CapsuleComponent|GetCapsuleHalfHeight (Variables|Default|GetCapsuleComponent)) -1.0) (.Z (Math|Vector|BreakVector Offset)))) false true)
  (Transformation|SetRelativeLocation _springarm (Math|Vector|MakeVector (.x _relativelocation) (.y _relativelocation) (* (.z (.boxextent (StaticMesh|GetBounds Mesh))) 2.0)) false true)
  (Rendering|Debug|DrawDebugSphere (Transformation|GetWorldLocation _springarm) 25.0 12 "(R=1.000000,G=1.000000,B=1.000000,A=1.000000)" 4.0))

(fn LockRotation
  (CallFunction|SLockRotation))