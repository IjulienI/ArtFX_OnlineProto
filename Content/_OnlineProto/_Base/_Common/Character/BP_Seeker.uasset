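; BP_Seeker is the Seeker character in an online prototype, who shoots Hider-tagged actors with a rifle.
; On BeginPlay it applies the skin mesh stored in the local GI_OnlineProto game instance.
; Shooting passes a camera-forward ray from a server-style event to a multicast-style one, which plays sound and runs a debug-drawn visibility trace.
; That same multicast-style event applies damage and spawns blood on Hider hits.
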(event Custom|MC_Shoot
  (params (Start :type Vector) (End :type Vector))
  (Audio|PlaySoundatLocation "/Game/Assets/Audio/CUE_Shoot.CUE_Shoot" (Transformation|GetWorldLocation (Variables|Default|GetSM_Wep_RifleBandit_01)) "0, 0, 0" 1.0 1.0 0.0 0 0 0 0)
  (bind (_outhit _returnvalue) (Collision|LineTraceByChannel Start End "TraceTypeQuery1" false 0 "ForDuration" true "(R=1.000000,G=0.000000,B=0.000000,A=1.000000)" "(R=0.000000,G=1.000000,B=0.000000,A=1.000000)" 2.0))
  (if _returnvalue
    (if (Actor|ActorHasTag (.HitActor (Collision|BreakHitResult _outhit)) "Hider")
      (Game|Damage|ApplyDamage (.HitActor (Collision|BreakHitResult _outhit)) 25.0 0 0)
      (Niagara|SpawnSystematLocation "/Game/_OnlineProto/_Base/VFX/NS_BloodSplash.NS_BloodSplash" (.ImpactPoint (Collision|BreakHitResult _outhit)) (Math|Conversions|RotationFromXVector (* (.ImpactNormal (Collision|BreakHitResult _outhit)) -1.0))))))

(event EventSShoot
  (bind _camera (Variables|Default|GetCamera))
  (bind _returnvalue (Transformation|GetWorldLocation _camera))
  (CallFunction|MCShoot _returnvalue (+ _returnvalue (* (Math|Vector|GetForwardVector _camera) 1e+04))))

(event EventBeginPlay
  (|CallParentFunction)
  (bind _asgi_online_proto (Utilities|Casting|CastToGI_OnlineProto (Game|GetGameInstance)))
  (Utilities|IsValid (.Skin (Utilities|Struct|BreakSTRUCT_Skin (Variables|/Game/_OnlineProto/_Base/_Common/_Managers/GI_OnlineProto.GI_OnlineProto_C|GetSkin _asgi_online_proto)))
    (:Is%20Valid
      (Components|SkeletalMesh|SetSkeletalMeshAsset (Variables|Character|GetMesh) (.Skin (Utilities|Struct|BreakSTRUCT_Skin (Variables|/Game/_OnlineProto/_Base/_Common/_Managers/GI_OnlineProto.GI_OnlineProto_C|GetSkin _asgi_online_proto)))))))

(fn ConstructionScript
  (|CallParentFunction))