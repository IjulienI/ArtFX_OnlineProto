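; BP_Healer is a healing actor that restores health to Hiders who touch it.
; On BeginPlay it checks the PS_Game of player state 0 and destroys itself if that player is a Seeker.
; Otherwise a slowed, replaying timeline bobs and spins the sphere.
; HitBox overlap with a "Hider"-tagged actor applies negative damage as healing, and the healer stays in place afterwards.
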(event OnComponentBeginOverlap(HitBox)
  (params (OverlappedComponent :type Primitive%20Component%20Object%20Reference) (OtherActor :type Actor%20Object%20Reference) (OtherComp :type Primitive%20Component%20Object%20Reference) (OtherBodyIndex :type Integer) (bFromSweep :type Boolean) (SweepResult :type Hit%20Result%20Structure%20%28by%20ref%29))
  (if (Actor|ActorHasTag OtherActor "Hider")
    (Game|Damage|ApplyDamage OtherActor -5e+01 0 0)))

(event Custom|Replay
  (bind _sphere (Variables|Default|GetSphere))
  (bind _relativerotation (Variables|/Script/Engine.SceneComponent|GetRelativeRotation _sphere))
  (bind (_direction _rotation _location) (Timeline|Movement PlayFromStart)
    (:Update
      (Transformation|SetRelativeLocation (Variables|Default|GetSphere) (Math|Vector|MakeVector 0.0 0.0 (Math|Float|Lerp 5e+01 65.0 _location)) false false)
      (Transformation|SetRelativeRotation _sphere (Math|Rotator|MakeRotator (.roll _relativerotation) (.pitch _relativerotation) (Math|Float|Lerp 0.0 359.0 _rotation)) false false))
    (:Finished
      (CallFunction|Replay))))

(event EventBeginPlay
  (bind _sphere (Variables|Default|GetSphere))
  (bind _relativerotation (Variables|/Script/Engine.SceneComponent|GetRelativeRotation _sphere))
  (bind _asps_game (Utilities|Casting|CastToPS_Game (Game|GetPlayerState 0)))
  (if (not (Variables|/Game/_OnlineProto/_Base/_Common/_Managers/PS_Game.PS_Game_C|GetbSeeker _asps_game))
    (Components|Timeline|SetPlayRate (Variables|Default|GetMovement) (/ 1.0 3.0))
    (bind (_direction _rotation _location) (Timeline|Movement PlayFromStart)
      (:Update
        (Transformation|SetRelativeLocation (Variables|Default|GetSphere) (Math|Vector|MakeVector 0.0 0.0 (Math|Float|Lerp 5e+01 65.0 _location)) false false)
        (Transformation|SetRelativeRotation _sphere (Math|Rotator|MakeRotator (.roll _relativerotation) (.pitch _relativerotation) (Math|Float|Lerp 0.0 359.0 _rotation)) false false))
      (:Finished
        (CallFunction|Replay)))
    (else
      (Actor|DestroyActor))))

(fn ConstructionScript)