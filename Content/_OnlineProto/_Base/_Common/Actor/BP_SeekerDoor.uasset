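; BP_SeekerDoor is a sliding double-door actor, apparently for the Seeker side of the online prototype.
; Its OpenDoor event plays a DoorMovement timeline, slowed to half speed at BeginPlay.
; Each update lerps the relative X of left and right corner and inside panels so they slide apart at a fixed height.
; It has no closing logic or trigger of its own, so another Blueprint must call OpenDoor.
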(event Custom|OpenDoor
  (bind _doormovement (Timeline|DoorMovement PlayFromStart)
    (:Update
      (Transformation|SetRelativeLocation (Variables|Default|GetLeftDoorCorner) (Math|Vector|MakeVector (Math|Float|Lerp 28.0 -12.0 _doormovement) 0.0 111.0) false false)
      (Transformation|SetRelativeLocation (Variables|Default|GetRightDoorCorner) (Math|Vector|MakeVector (Math|Float|Lerp 195.0 235.0 _doormovement) 0.0 111.0) false false)
      (Transformation|SetRelativeLocation (Variables|Default|GetLeftDoorInside) (Math|Vector|MakeVector (Math|Float|Lerp 84.0 -1e+01 _doormovement) 0.0 111.0) false false)
      (Transformation|SetRelativeLocation (Variables|Default|GetRightDoorInside) (Math|Vector|MakeVector (Math|Float|Lerp 1.4e+02 233.0 _doormovement) 0.0 111.0) false false))))

(event EventBeginPlay
  (Components|Timeline|SetPlayRate (Variables|Default|GetDoorMovement) (/ 1.0 2.0)))

(event Collision|EventActorBeginOverlap
  (params (OtherActor :type Actor%20Object%20Reference)))

(event EventTick
  (params (DeltaSeconds :type Float%20%28single-precision%29)))

(fn ConstructionScript)