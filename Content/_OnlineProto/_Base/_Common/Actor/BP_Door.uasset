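; BP_Door is an interactable door actor meant to swing open and closed through a timeline.
; BeginPlay scales the DoorMovement timeline's play rate by RotationDuration.
; Interact stores the investigator, flips the Open flag, and reverses the timeline when open or plays it otherwise.
; The timeline update sets the door's world yaw to a fixed zero, as the Lerp on the Move track is unused.
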(event EventBeginPlay
  (Components|Timeline|SetPlayRate (Variables|Default|GetDoorMovement) (/ 1.0 (Variables|Default|GetRotationDuration))))

(event EventInteract
  (params (Investigator :type BP%20Base%20Character%20Object%20Reference))
  (bind _door (Variables|Default|GetDoor))
  (bind _returnvalue (Transformation|GetWorldRotation _door))
  (Variables|Default|SetPlayer Investigator)
  (bind _output_get (Variables|Default|SetbOpen (not (Variables|Default|GetbOpen))))
  (if _output_get
    (bind _move (Timeline|DoorMovement Reverse)
      (:Update
        (Transformation|SetWorldRotation (Variables|Default|GetDoor) (Math|Rotator|MakeRotator (.roll _returnvalue) (.pitch _returnvalue) 0.0) false false)))
    (else
      (Timeline|DoorMovement Play))))

(fn ConstructionScript)